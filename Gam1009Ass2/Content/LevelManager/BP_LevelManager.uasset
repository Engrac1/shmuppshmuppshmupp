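; Level manager that spawns enemies and powerups around the player on looping timers and starts the theme music.
; Enemy waves swap in a big enemy by spawn-count modulus and grow when the total hits a threshold multiple.
; Spawn points add scaled offsets from a random stream to the player's location.
; StopSpawns clears both timers; powerups always get Firerate, as the random powerup selector is never called.
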(event Custom|BeginEnemySpawning
  (CallFunction|StartSpawningEnemy))

(event Custom|BeginPowerupSpawning
  (CallFunction|SpawnPowerup))

(event EventBeginPlay
  (Class|KismetMathLibrary|SeedRandomStream (Variables|Default|GetRandomStream))
  (CallFunction|StartSpawningEnemy)
  (bind _returnvalue (Utilities|Time|SetTimerbyEvent (delegate Custom|BeginEnemySpawning) (Variables|Default|GetEnemySpawnInterval) true))
  (Variables|Default|SetEnemySpawnTimer _returnvalue)
  (bind _returnvalue_2 (Utilities|Time|SetTimerbyEvent (delegate Custom|BeginPowerupSpawning) (Variables|Default|GetPowerupSpawnInterval) true))
  (Variables|Default|SetPowerup%20Spawn%20Timer _returnvalue_2)
  (Audio|SpawnSoundAttached "/Game/Sounds/Music/DST-TowerDefenseTheme.DST-TowerDefenseTheme" (Variables|/Script/Engine.Actor|GetRootComponent (Game|GetPlayerCharacter 0)) "None" "0, 0, 0" "0, 0, 0" "KeepRelativeOffset" false 1.0 1.0 0.0 0 0))

(event EventStopSpawns
  (Utilities|Time|ClearandInvalidateTimerbyHandle (Variables|Default|GetEnemySpawnTimer))
  (Utilities|Time|ClearandInvalidateTimerbyHandle (Variables|Default|GetPowerup%20Spawn%20Timer)))

(fn ConstructionScript)

(fn StartSpawningEnemy
  (for _index (range 1 (Variables|Default|GetEnemiesToSpawn))
    (bind _selection (CallFunction|SelectEnemytoSpawn))
    (CallFunction|PlaceEnemyinWorld _selection)
    (Math|Integer|IncrementInt (Variables|Default|GetEnemy%20Spawns%20Done)))
  (CallFunction|IncrementSpawnDifficulty))

(fn SpawnPowerup
  (bind _returnvalue (CallFunction|GetSpawnLocation (Variables|Default|GetRandomStream)))
  (bind _returnvalue_2 (Game|SpawnActorfromClass "/Game/Blueprints/BP_Powerup.BP_Powerup_C" _returnvalue "Undefined" "MultiplyWithRoot" 0 0))
  (CallFunction|SetPowerupSpawnProperties _returnvalue_2 "NewEnumerator0"))

(fn GetSpawnLocation
  (params (Stream :type Random%20Stream%20Structure))
  (bind _returnvalue (Class|KismetMathLibrary|RandomIntegerfromStream Stream 10))
  (bind _returnvalue_2 (Game|GetPlayerCharacter 0))
  (bind _spawndistancemodifier (Variables|Default|GetSpawnDistanceModifier))
  (bind _returnvalue_3 (Transformation|GetActorLocation _returnvalue_2))
  (bind _returnvalue_4 (Utilities|Select :Index _returnvalue :Option%200 "1.000000,1.000000,0.000000" :Option%201 "1.000000,-1.000000,0.000000" :Option%202 "-1.000000,1.000000,0.000000" :Option%203 "-1.000000,-1.000000,0.000000" :Option%204 "0.750000,1.000000,0.000000" :Option%205 "1.000000,0.750000,0.000000" :Option%206 "-0.750000,1.000000,0.000000" :Option%207 "1.000000,-0.750000,0.000000" :Option%208 "-0.750000,-1.000000,0.000000" :Option%209 "-1.000000,-0.750000,0.000000"))
  (bind _returnvalue_5 (* _returnvalue_4 _spawndistancemodifier))
  (bind _returnvalue_6 (+ _returnvalue_3 _returnvalue_5))
  ;[1 1 1] Gets a random spawn location, derived from the player's current location. Increasing SpawnDistanceModifier will make enemies spawn further away from the player.
  (return (Math|Transform|MakeTransform (Math|Vector|MakeVector (.x _returnvalue_6) (.y _returnvalue_6) (.z (Transformation|GetActorLocation (Game|GetPlayerCharacter 0)))))))

(fn PlaceEnemyinWorld
  (params (EnemyToSpawn :type Actor%20Class%20Reference))
  (bind _returnvalue (CallFunction|GetSpawnLocation (Variables|Default|GetRandomStream)))
  (Game|SpawnActorfromClass EnemyToSpawn _returnvalue "Undefined" "MultiplyWithRoot" 0 0)
  (Class|KismetMathLibrary|SeedRandomStream (Variables|Default|GetRandomStream)))

(fn SelectEnemytoSpawn
  ;[1 1 1] Takes the modulus of the amount of enemies spawned, to determine what enemy to spawn. This way, every "X enemy spawn modulus" enemy spawned is that enemy type.
  (if (and (== (Math|Integer|%(Integer) (Variables|Default|GetEnemy%20Spawns%20Done) (Variables|Default|GetBig%20Enemy%20Spawn%20Modulus)) 0) (!= (Variables|Default|GetEnemy%20Spawns%20Done) 0))
    (return "/Game/Enemies/BP_BigEnemy.BP_BigEnemy_C")
    (else
      (return "/Game/Enemies/BP_EnemyBasic.BP_EnemyBasic_C"))))

(fn IncrementSpawnDifficulty
  (if (== (Math|Integer|%(Integer) (Variables|Default|GetEnemy%20Spawns%20Done) (Variables|Default|GetEnemy%20Spawn%20Increase%20Threshold)) 0)
    (Variables|Default|SetEnemiesToSpawn (+ (Variables|Default|GetEnemiesToSpawn) (Variables|Default|GetEnemySpawnsDifficultyIncreaseAmount)))))

(fn SetPowerupSpawnProperties
  (params (Powerup :type BP%20Powerup%20Object%20Reference) (PowerupInput :type E_Powerups%20Enum :default "NewEnumerator0"))
  (switch Utilities|FlowControl|Switch|SwitchonE_Powerups PowerupInput
    (:NewEnumerator0
      (Variables|/Game/Blueprints/BP_Powerup.BP_Powerup_C|SetFlashMaterial Powerup "/Game/Materials/M_Firerate.M_Firerate"))
    (:NewEnumerator1
      (Variables|/Game/Blueprints/BP_Powerup.BP_Powerup_C|SetFlashMaterial Powerup "/Game/Materials/M_Health.M_Health"))
    (:NewEnumerator2
      (Variables|/Game/Blueprints/BP_Powerup.BP_Powerup_C|SetFlashMaterial Powerup "/Game/Materials/M_WipeCharge.M_WipeCharge"))))

(fn SelectPoweruptoSpawn
  (switch int (Math|Random|RandomIntegerinRangefromStream (Variables|Default|GetRandomStream) 0 3)
    (:0
      _)
    (:1
      _)
    (:2
      _)
    (:3
      (return "NewEnumerator0"))
    (:4
      (return "NewEnumerator2"))
    (:5
      (return "NewEnumerator2")))
  (return "NewEnumerator1"))