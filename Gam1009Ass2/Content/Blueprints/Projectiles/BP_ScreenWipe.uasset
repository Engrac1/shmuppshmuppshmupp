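; A screen-wipe projectile that damages enemies across a growing area.
; Each tick a Box component grows horizontally by a fixed step, independent of frame time, while its height stays constant.
; Enemies overlapping the box take instakill damage if tagged CanBeWiped, otherwise a separate damage amount meant for immune targets.
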(event OnComponentBeginOverlap(Box)
  (params (OverlappedComponent :type Primitive%20Component%20Object%20Reference) (OtherActor :type Actor%20Object%20Reference) (OtherComp :type Primitive%20Component%20Object%20Reference) (OtherBodyIndex :type Integer) (bFromSweep :type Boolean) (SweepResult :type Hit%20Result%20Structure%20%28by%20ref%29))
  (if (Actor|ActorHasTag OtherActor "Enemy")
    (Game|Damage|ApplyDamage OtherActor (Math|Float|SelectFloat (Variables|Default|GetInstakillDamage) (Variables|Default|GetScreenWipeDamageVSImmune) (Actor|ActorHasTag OtherActor "CanBeWiped")) 0 0)))

(event EventTick
  (params (DeltaSeconds :type Float%20%28single-precision%29))
  (bind _box (Variables|Default|GetBox))
  (bind _returnvalue (Transformation|GetWorldScale _box))
  (Transformation|SetWorldScale3D _box (Math|Vector|MakeVector (+ (.x _returnvalue) 0.28) (+ (.y _returnvalue) 0.28) (.z _returnvalue))))

(fn ConstructionScript)