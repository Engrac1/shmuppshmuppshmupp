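; BP_PlayerProjectile is a player projectile that damages actors it hits.
; On Hit, it applies ProjectileDamage to actors tagged Enemy and destroys itself, ignoring anything else.
; An unfinished "kill on sleep" is disconnected: its looping timer never runs, and its check would destroy the projectile while velocity is above zero rather than when stopped.
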(event Custom|CustomEvent
  ;[1 1 1] Theoretical kill on sleep, not currently functioning.
  (if (> (Math|Vector|VectorLength (Variables|/Script/Engine.MovementComponent|GetVelocity (Variables|Default|GetProjectileMovement))) 0.0)
    (Actor|DestroyActor)))

(event EventBeginPlay
  ;[1 1 1] Theoretical kill on sleep, not currently functioning.
)

(event Collision|EventHit
  (params (MyComp :type Primitive%20Component%20Object%20Reference) (Other :type Actor%20Object%20Reference) (OtherComp :type Primitive%20Component%20Object%20Reference) (bSelfMoved :type Boolean) (HitLocation :type Vector :default "0, 0, 0") (HitNormal :type Vector :default "0, 0, 0") (NormalImpulse :type Vector :default "0, 0, 0") (Hit :type Hit%20Result%20Structure%20%28by%20ref%29))
  (if (Actor|ActorHasTag Other "Enemy")
    (Game|Damage|ApplyDamage Other (Variables|Default|GetProjectileDamage) 0 0)
    (Actor|DestroyActor)))

(fn ConstructionScript)