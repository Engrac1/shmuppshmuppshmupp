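; BP_BigEnemy is an enemy that damages the player on contact and destroys itself in the process.
; Incoming damage goes through ACHealth, which triggers death when its handler returns true.
; Die spawns a hurt or death Niagara effect and updates the player's score message, passing the kill score only for self-kills on contact.
; Random hit and death sound helpers are defined but not called here.
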(event Collision|EventHit
  (params (MyComp :type Primitive%20Component%20Object%20Reference) (Other :type Actor%20Object%20Reference) (OtherComp :type Primitive%20Component%20Object%20Reference) (bSelfMoved :type Boolean) (HitLocation :type Vector :default "0, 0, 0") (HitNormal :type Vector :default "0, 0, 0") (NormalImpulse :type Vector :default "0, 0, 0") (Hit :type Hit%20Result%20Structure%20%28by%20ref%29))
  (bind _returnvalue (Game|GetPlayerCharacter 0))
  (if (== Other _returnvalue)
    (Game|Damage|ApplyDamage _returnvalue (Variables|Default|GetDamage) 0 0)
    (CallFunction|Die true)))

(event Game|Damage|EventAnyDamage
  (params (Damage :type Float%20%28single-precision%29) (DamageType :type Damage%20Type%20Object%20Reference) (InstigatedBy :type Controller%20Object%20Reference) (DamageCauser :type Actor%20Object%20Reference))
  (bind _isdead_ (Default|HandleDamage (Variables|Default|GetAC_Health) Damage))
  (if _isdead_
    (CallFunction|Die false)))

(fn ConstructionScript)

(fn Die
  (params (KilledSelf? :type Boolean))
  (Niagara|SpawnSystematLocation (select KilledSelf? "/Game/Niagara/NS_PlayerHurt.NS_PlayerHurt" "/Game/Niagara/NS_EnemyDeath.NS_EnemyDeath") (Transformation|GetActorLocation))
  (Class|BIUIUpdates|UpdateScore(Message) (Game|GetPlayerCharacter 0) (Math|Integer|SelectInt (Variables|Default|GetScoreGrantedOnKill) 0 KilledSelf?))
  (Actor|DestroyActor))

(fn PlayDeathSound
  (Audio|PlaySoundatLocation (.OutItem (Utilities|Array|Random (Variables|Default|GetDeathSounds))) (Transformation|GetActorLocation) "0, 0, 0" 1.0 1.0 0.0 0 0 0 0))

(fn PlayHitSound
  (Audio|PlaySoundatLocation (.OutItem (Utilities|Array|Random (Variables|Default|GetHitSounds))) (Transformation|GetActorLocation) "0, 0, 0" 1.0 1.0 0.0 0 0 0 0))