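; Basic enemy that damages the player on contact and destroys itself, or dies when its health component reports lethal damage.
; A looping timer switches between normal and gap-close walk speed, intended to keep enemies near the screen edge.
; A shared Die function spawns Niagara effects and messages the player to award score and wipe charge, or drain charge after contact.
; Damage plays random hit or death sounds, with very large killing blows staying silent.
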(event Custom|SetSpeed
  ;[1 1 1] Makes sure that the player can't just keep running, by making sure enemies are always close to the screen edge. Uses a timer because this check does not need to occur on tick, and thus is better for performance.
  (Variables|/Script/Engine.CharacterMovementComponent|SetMaxWalkSpeed (Variables|Character|GetCharacterMovement) (select (Utilities|ShouldbeGapCloseSpeed?) (Variables|Default|GetGapCloseSpeed) (Variables|Default|GetSpeed))))

(event Collision|EventHit
  (params (MyComp :type Primitive%20Component%20Object%20Reference) (Other :type Actor%20Object%20Reference) (OtherComp :type Primitive%20Component%20Object%20Reference) (bSelfMoved :type Boolean) (HitLocation :type Vector :default "0, 0, 0") (HitNormal :type Vector :default "0, 0, 0") (NormalImpulse :type Vector :default "0, 0, 0") (Hit :type Hit%20Result%20Structure%20%28by%20ref%29))
  (bind _returnvalue (Game|GetPlayerCharacter 0))
  (if (== Other _returnvalue)
    (Game|Damage|ApplyDamage _returnvalue (Variables|Default|GetDamage) 0 0)
    (CallFunction|Die true)))

(event EventBeginPlay
  ;[1 1 1] Makes sure that the player can't just keep running, by making sure enemies are always close to the screen edge. Uses a timer because this check does not need to occur on tick, and thus is better for performance.
  (Utilities|Time|SetTimerbyEvent (delegate Custom|SetSpeed) 0.5 true))

(event Game|Damage|EventAnyDamage
  (params (Damage :type Float%20%28single-precision%29) (DamageType :type Damage%20Type%20Object%20Reference) (InstigatedBy :type Controller%20Object%20Reference) (DamageCauser :type Actor%20Object%20Reference))
  (bind _isdead_ (Default|HandleDamage (Variables|Default|GetAC_Health) Damage))
  (if _isdead_
    (if (> Damage 3e+02)
      (CallFunction|Die false)
      (else
        (CallFunction|PlayDeathSound)
        (CallFunction|Die false)))
    (else
      (CallFunction|PlayHitSound))))

(fn ConstructionScript)

(fn Die
  (params (KilledSelf? :type Boolean))
  (bind _returnvalue (Game|GetPlayerCharacter 0))
  (Niagara|SpawnSystematLocation (select KilledSelf? "/Game/Niagara/NS_PlayerHurt.NS_PlayerHurt" "/Game/Niagara/NS_EnemyDeath.NS_EnemyDeath") (Transformation|GetActorLocation))
  (Class|BIUIUpdates|UpdateScore(Message) _returnvalue (Math|Integer|SelectInt 0 (Variables|Default|GetScore%20Granted%20on%20Kill) KilledSelf?))
  (Class|BIPlayer|ChangeWipeCharge(Message) _returnvalue (Math|Float|SelectFloat (Variables|Default|GetChargeToDrainOnHit) (Variables|Default|GetEnemyChargeValue) KilledSelf?))
  (Actor|DestroyActor))

(fn PlayHitSound
  (Audio|PlaySoundatLocation (.OutItem (Utilities|Array|Random (Variables|Default|GetHitSound))) (Transformation|GetActorLocation) "0, 0, 0" 1.0 1.0 0.0 0 0 0 0))

(fn PlayDeathSound
  (Audio|PlaySoundatLocation (.OutItem (Utilities|Array|Random (Variables|Default|GetDeathSound))) (Transformation|GetActorLocation) "0, 0, 0" 1.0 1.0 0.0 0 0 0 0))