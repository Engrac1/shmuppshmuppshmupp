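; BP_Powerup is a pickup actor that grants its configured powerup to the player for a set duration.
; On BeginPlay a looping timer makes the mesh blink by briefly swapping to a flash material, then back to the base material halfway through each interval.
; When hit by the first player's character, it sends that character an ActivatePowerup message with the powerup and duration, then destroys itself.
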(event Custom|Flash
  (Rendering|Material|SetMaterial (Variables|Default|GetPowerupMesh) 0 (Variables|Default|GetFlashMaterial))
  (Utilities|FlowControl|Delay (/ (Variables|Default|GetFlashInterval) 2.0))
  (Rendering|Material|SetMaterial (Variables|Default|GetPowerupMesh) 0 "/Game/Materials/M_PowerupBase.M_PowerupBase"))

(event EventBeginPlay
  (Utilities|Time|SetTimerbyEvent (delegate Custom|Flash) (Variables|Default|GetFlashInterval) true))

(event Collision|EventHit
  (params (MyComp :type Primitive%20Component%20Object%20Reference) (Other :type Actor%20Object%20Reference) (OtherComp :type Primitive%20Component%20Object%20Reference) (bSelfMoved :type Boolean) (HitLocation :type Vector :default "0, 0, 0") (HitNormal :type Vector :default "0, 0, 0") (NormalImpulse :type Vector :default "0, 0, 0") (Hit :type Hit%20Result%20Structure%20%28by%20ref%29))
  (if (== Other (Game|GetPlayerCharacter 0))
    (Class|BIPlayer|ActivatePowerup(Message) (Game|GetPlayerCharacter 0) (Variables|Default|GetPowerupDuration) (Variables|Default|GetPowerup))
    (Actor|DestroyActor)))

(fn ConstructionScript)