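; BP_ScreenWipe is a screen-wipe attack actor that damages enemies caught in an expanding sphere.
; A looping timer grows the sphere radius linearly, scaling each step from the tick interval, the actor's initial lifespan and the maximum size.
; Overlapping actors tagged Enemy take instakill damage if also tagged CanBeWiped, otherwise a separate damage amount for immune targets.
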(event OnComponentBeginOverlap(Sphere)
  (params (OverlappedComponent :type Primitive%20Component%20Object%20Reference) (OtherActor :type Actor%20Object%20Reference) (OtherComp :type Primitive%20Component%20Object%20Reference) (OtherBodyIndex :type Integer) (bFromSweep :type Boolean) (SweepResult :type Hit%20Result%20Structure%20%28by%20ref%29))
  (if (Actor|ActorHasTag OtherActor "Enemy")
    (Game|Damage|ApplyDamage OtherActor (Math|Float|SelectFloat (Variables|Default|GetInstakillDamage) (Variables|Default|GetScreenWipeDamageVSImmune) (Actor|ActorHasTag OtherActor "CanBeWiped")) 0 0)))

(event Custom|UpdateSphereRadius
  (Components|Sphere|SetSphereRadius (Variables|Default|GetSphere) (CallFunction|GetNewSphereRadius) true))

(event EventBeginPlay
  (Utilities|Time|SetTimerbyEvent (delegate Custom|UpdateSphereRadius) (Variables|Default|GetIncrementToScale) true))

(fn ConstructionScript)

(fn GetNewSphereRadius
  (return (+ (Variables|/Script/Engine.SphereComponent|GetSphereRadius (Variables|Default|GetSphere)) (* (/ (Variables|Default|GetIncrementToScale) (Variables|Actor|GetInitialLifeSpan)) (Variables|Default|GetSphereMaxSize)))))