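; BP_EnemyProjectile is an enemy projectile actor that damages what it hits and can itself be destroyed by damage.
; A looping timer set on BeginPlay makes the mesh flash by swapping between two materials, switching back halfway through each interval.
; On hit it applies damage to the other actor and destroys itself, while taking any damage spawns a Niagara destruction effect before destroying it.
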(event Custom|CustomEvent
  (Rendering|Material|SetMaterial (Variables|Default|GetProjectileMesh) 0 "/Game/Materials/M_EnemyProjectileFlash.M_EnemyProjectileFlash")
  (Utilities|FlowControl|Delay (/ (Variables|Default|GetFlashInterval) 2.0))
  (Rendering|Material|SetMaterial (Variables|Default|GetProjectileMesh) 0 "/Game/Materials/M_DamageFlash.M_DamageFlash"))

(event EventBeginPlay
  (Utilities|Time|SetTimerbyEvent (delegate Custom|CustomEvent) (Variables|Default|GetFlashInterval) true))

(event Game|Damage|EventAnyDamage
  (params (Damage :type Float%20%28single-precision%29) (DamageType :type Damage%20Type%20Object%20Reference) (InstigatedBy :type Controller%20Object%20Reference) (DamageCauser :type Actor%20Object%20Reference))
  (Niagara|SpawnSystematLocation "/Game/Niagara/NS_EnemyProjectileDestroyed.NS_EnemyProjectileDestroyed" (Transformation|GetActorLocation))
  (Actor|DestroyActor))

(event Collision|EventHit
  (params (MyComp :type Primitive%20Component%20Object%20Reference) (Other :type Actor%20Object%20Reference) (OtherComp :type Primitive%20Component%20Object%20Reference) (bSelfMoved :type Boolean) (HitLocation :type Vector :default "0, 0, 0") (HitNormal :type Vector :default "0, 0, 0") (NormalImpulse :type Vector :default "0, 0, 0") (Hit :type Hit%20Result%20Structure%20%28by%20ref%29))
  (Game|Damage|ApplyDamage Other (Variables|Default|GetProjectileDamage) 0 0)
  (Actor|DestroyActor))

(fn ConstructionScript)