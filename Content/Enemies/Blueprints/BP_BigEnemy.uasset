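; Big enemy that damages the player on contact and destroys itself, or dies when its health component reports a lethal hit.
; Non-lethal damage spawns a Niagara burst just in front of it.
; Die picks effects by cause, messaging the player with score and wipe charge for kills, or zero score and a charge drain for contact deaths.
; It then breaks a geometry collection at the cube's transform before destroying the actor.
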(event Collision|EventHit
  (params (MyComp :type Primitive%20Component%20Object%20Reference) (Other :type Actor%20Object%20Reference) (OtherComp :type Primitive%20Component%20Object%20Reference) (bSelfMoved :type Boolean) (HitLocation :type Vector :default "0, 0, 0") (HitNormal :type Vector :default "0, 0, 0") (NormalImpulse :type Vector :default "0, 0, 0") (Hit :type Hit%20Result%20Structure%20%28by%20ref%29))
  (if (== Other (Game|GetPlayerCharacter 0))
    (Game|Damage|ApplyDamage Other (Variables|Default|GetDamage) 0 0)
    (CallFunction|Die true)))

(event Game|Damage|EventAnyDamage
  (params (Damage :type Float%20%28single-precision%29) (DamageType :type Damage%20Type%20Object%20Reference) (InstigatedBy :type Controller%20Object%20Reference) (DamageCauser :type Actor%20Object%20Reference))
  (bind _isdead_ (Default|HandleDamage (Variables|Default|GetAC_Health) Damage))
  (if _isdead_
    (CallFunction|Die false)
    (else
      (Niagara|SpawnSystematLocation "/Game/Niagara/NS_EnemyDeath.NS_EnemyDeath" (+ (Transformation|GetActorLocation) (* (Transformation|GetActorForwardVector) 1e+01))))))

(fn ConstructionScript)

(fn Die
  (params (KilledSelf? :type Boolean))
  (bind _returnvalue (Game|GetPlayerCharacter 0))
  (Niagara|SpawnSystematLocation (select KilledSelf? "/Game/Niagara/NS_PlayerHurt.NS_PlayerHurt" "/Game/Niagara/NS_EnemyDeath.NS_EnemyDeath") (Transformation|GetActorLocation))
  (Class|BIUIUpdates|UpdateScore(Message) _returnvalue (Math|Integer|SelectInt 0 (Variables|Default|GetScore%20Granted%20on%20Kill) KilledSelf?))
  (Class|BIPlayer|ChangeWipeCharge(Message) _returnvalue (Math|Float|SelectFloat (Variables|Default|GetChargeToDrainOnHit) (Variables|Default|GetEnemyChargeValue) KilledSelf?))
  (Utilities|SpawnandBreakGeoCollection "/Game/Materials/M_BigEnemy.M_BigEnemy" (Transformation|GetWorldTransform (Variables|Default|GetCube))
    (:ExecOut
      (Actor|DestroyActor))))

(fn PlayDeathSound
  (Audio|PlaySoundatLocation (.OutItem (Utilities|Array|Random (Variables|Default|GetDeathSounds))) (Transformation|GetActorLocation) "0, 0, 0" 1.0 1.0 0.0 0 0 0 0))

(fn PlayHitSound
  (Audio|PlaySoundatLocation (.OutItem (Utilities|Array|Random (Variables|Default|GetHitSounds))) (Transformation|GetActorLocation) "0, 0, 0" 1.0 1.0 0.0 0 0 0 0))