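; Level manager that spawns enemies, powerups and weapon-upgrade minibosses around the player and starts the theme music.
; Looping timers drive each spawn type, placing actors at random stream-picked offsets from the player until StopSpawns clears them.
; Spawn-count modulus picks boss, big, shooting or basic enemies, while wave and rushdown sizes grow over time.
; Minibosses receive successive upgrades to drop, and events spawn powerup or upgrade pickups at given transforms.
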(event Custom|BeginEnemySpawning
  (CallFunction|StartSpawningEnemy))

(event Custom|BeginPowerupSpawning
  (bind _returnvalue (CallFunction|GetSpawnLocation (Variables|Default|GetRandomStream)))
  (CallFunction|SpawnPowerup _returnvalue))

(event Custom|RushdownEnemy
  (CallFunction|RushdownPlayer))

(event Custom|WeaponUpgradeEnemySpawn
  (bind _spawnedenemy (CallFunction|SpawnUpgradeEnemy))
  (bind _outputfiringmode (CallFunction|GetWeaponUpgradetoSpawn))
  (Variables|/Game/Enemies/Blueprints/BP_Miniboss.BP_Miniboss_C|SetUpgradeToDrop _spawnedenemy _outputfiringmode)
  (Math|Integer|IncrementInt (Variables|Default|GetUpgradeIncrement)))

(event EventBeginPlay
  (Class|KismetMathLibrary|SeedRandomStream (Variables|Default|GetRandomStream))
  (CallFunction|StartSpawningEnemy)
  (bind _returnvalue (Utilities|Time|SetTimerbyEvent (delegate Custom|BeginEnemySpawning) (Variables|EnemySpawning|GetEnemySpawnInterval) true))
  (Variables|EnemySpawning|SetEnemySpawnTimer _returnvalue)
  (bind _returnvalue_2 (Utilities|Time|SetTimerbyEvent (delegate Custom|BeginPowerupSpawning) (Variables|Default|GetPowerupSpawnInterval) true))
  (Variables|Default|SetPowerup%20Spawn%20Timer _returnvalue_2)
  (Audio|SpawnSoundAttached "/Game/Sounds/Music/DST-TowerDefenseTheme.DST-TowerDefenseTheme" (Variables|/Script/Engine.Actor|GetRootComponent (Game|GetPlayerCharacter 0)) "None" "0, 0, 0" "0, 0, 0" "KeepRelativeOffset" false 1.0 1.0 0.0 0 0)
  (bind _returnvalue_3 (Utilities|Time|SetTimerbyEvent (delegate Custom|RushdownEnemy) (Variables|RushdownEnemySpawning|GetRushdownEnemyTimer) true))
  (Variables|RushdownEnemySpawning|SetRushdownTimer _returnvalue_3)
  (bind _returnvalue_4 (Utilities|Time|SetTimerbyEvent (delegate Custom|WeaponUpgradeEnemySpawn) (Variables|Default|GetWeaponEnemySpawnInterval) true))
  (Variables|Default|SetUpgradeEnemyTimer _returnvalue_4))

(event EventSpawnPowerupBasicEnemy
  (params (Transform :type Transform))
  (CallFunction|SpawnPowerup Transform))

(event EventSpawnWeaponUpgrade
  (params (Transform :type Transform) (Upgrade :type E_FiringModes%20Enum :default "NewEnumerator0"))
  (bind _upgradepickup (CallFunction|PlaceWeaponUpgrade Transform))
  (Variables|/Game/Blueprints/BP_WeaponUpgrade.BP_WeaponUpgrade_C|SetWeaponUpgrade _upgradepickup Upgrade))

(event EventStopSpawns
  (Utilities|Time|ClearandInvalidateTimerbyHandle (Variables|EnemySpawning|GetEnemySpawnTimer))
  (Utilities|Time|ClearandInvalidateTimerbyHandle (Variables|Default|GetPowerup%20Spawn%20Timer))
  (Utilities|Time|ClearandInvalidateTimerbyHandle (Variables|RushdownEnemySpawning|GetRushdownTimer))
  (Utilities|Time|ClearandInvalidateTimerbyHandle (Variables|Default|GetUpgradeEnemyTimer)))

(fn ConstructionScript)

(fn StartSpawningEnemy
  (for _index (range 0 (Variables|EnemySpawning|GetEnemiesToSpawn))
    (bind _selection (CallFunction|SelectEnemytoSpawn (Variables|EnemySpawning|GetEnemy%20Spawns%20Done)))
    (CallFunction|PlaceEnemyinWorld _selection)
    (Math|Integer|IncrementInt (Variables|EnemySpawning|GetEnemy%20Spawns%20Done)))
  (CallFunction|IncrementSpawnDifficulty))

(fn SpawnPowerup
  (params (Transform :type Transform))
  (bind _returnvalue (Game|SpawnActorfromClass "/Game/Blueprints/BP_Powerup.BP_Powerup_C" Transform "Undefined" "MultiplyWithRoot" 0 0))
  (CallFunction|SetPowerupSpawnProperties _returnvalue "NewEnumerator0"))

(fn GetSpawnLocation
  (params (Stream :type Random%20Stream%20Structure))
  (bind _returnvalue (Class|KismetMathLibrary|RandomIntegerfromStream Stream 10))
  (bind _returnvalue_2 (Game|GetPlayerCharacter 0))
  (bind _spawndistancemodifier (Variables|EnemySpawning|GetSpawnDistanceModifier))
  (bind _returnvalue_3 (Transformation|GetActorLocation _returnvalue_2))
  (bind _returnvalue_4 (Utilities|Select :Index _returnvalue :Option%200 "1.000000,1.000000,0.000000" :Option%201 "1.000000,-1.000000,0.000000" :Option%202 "-1.000000,1.000000,0.000000" :Option%203 "-1.000000,-1.000000,0.000000" :Option%204 "0.750000,1.000000,0.000000" :Option%205 "1.000000,0.750000,0.000000" :Option%206 "-0.750000,1.000000,0.000000" :Option%207 "1.000000,-0.750000,0.000000" :Option%208 "-0.750000,-1.000000,0.000000" :Option%209 "-1.000000,-0.750000,0.000000"))
  (bind _returnvalue_5 (* _returnvalue_4 _spawndistancemodifier))
  (bind _returnvalue_6 (+ _returnvalue_3 _returnvalue_5))
  ;[1 1 1] Gets a random spawn location, derived from the player's current location. Increasing SpawnDistanceModifier will make enemies spawn further away from the player.
  (return (Math|Transform|MakeTransform (Math|Vector|MakeVector (.x _returnvalue_6) (.y _returnvalue_6) (.z (Transformation|GetActorLocation (Game|GetPlayerCharacter 0)))))))

(fn PlaceEnemyinWorld
  (params (EnemyToSpawn :type Actor%20Class%20Reference))
  (bind _returnvalue (CallFunction|GetSpawnLocation (Variables|Default|GetRandomStream)))
  (bind _returnvalue_2 (Game|SpawnActorfromClass EnemyToSpawn _returnvalue "Undefined" "MultiplyWithRoot" 0 0))
  (Class|KismetMathLibrary|SeedRandomStream (Variables|Default|GetRandomStream))
  (return _returnvalue_2))

(fn SelectEnemytoSpawn
  (params (SpawnIndex :type Integer))
  ;[1 1 1] Takes the modulus of the amount of enemies spawned, to determine what enemy to spawn. This way, every "X enemy spawn modulus" enemy spawned is that enemy type.
  (if (Utilities|CompareModulustoEnemiesSpawned SpawnIndex (Variables|Default|GetBossEnemySpawnModulus))
    (return "/Game/Enemies/Blueprints/BP_BossEnemy.BP_BossEnemy_C")
    (elif (Utilities|CompareModulustoEnemiesSpawned SpawnIndex (Variables|EnemySpawning|GetBig%20Enemy%20Spawn%20Modulus))
      (return "/Game/Enemies/Blueprints/BP_BigEnemy.BP_BigEnemy_C")
      (elif (Utilities|CompareModulustoEnemiesSpawned SpawnIndex (Variables|EnemySpawning|GetShootingEnemySpawnModulus))
        (return "/Game/Enemies/Blueprints/BP_ShootingEnemy.BP_ShootingEnemy_C")
        (else
          (return "/Game/Enemies/Blueprints/BP_EnemyBasic.BP_EnemyBasic_C"))))))

(fn IncrementSpawnDifficulty
  (if (== (Math|Integer|%(Integer) (Variables|EnemySpawning|GetEnemy%20Spawns%20Done) (Variables|EnemySpawning|GetEnemy%20Spawn%20Increase%20Threshold)) 0)
    (Variables|EnemySpawning|SetEnemiesToSpawn (+ (Variables|EnemySpawning|GetEnemiesToSpawn) (Variables|EnemySpawning|GetEnemySpawnsDifficultyIncreaseAmount)))))

(fn SetPowerupSpawnProperties
  (params (Powerup :type BP%20Powerup%20Object%20Reference) (PowerupInput :type E_Powerups%20Enum :default "NewEnumerator0"))
  (switch Utilities|FlowControl|Switch|SwitchonE_Powerups PowerupInput
    (:NewEnumerator0
      (Variables|/Game/Blueprints/BP_Powerup.BP_Powerup_C|SetFlashMaterial Powerup "/Game/Materials/M_Firerate.M_Firerate"))
    (:NewEnumerator1
      (Variables|/Game/Blueprints/BP_Powerup.BP_Powerup_C|SetFlashMaterial Powerup "/Game/Materials/M_Health.M_Health"))
    (:NewEnumerator2
      (Variables|/Game/Blueprints/BP_Powerup.BP_Powerup_C|SetFlashMaterial Powerup "/Game/Materials/M_WipeCharge.M_WipeCharge"))))

(fn SelectPoweruptoSpawn
  (switch int (Math|Random|RandomIntegerinRangefromStream (Variables|Default|GetRandomStream) 0 5)
    (:0
      _)
    (:1
      _)
    (:2
      _)
    (:3
      (return "NewEnumerator0"))
    (:4
      (return "NewEnumerator2"))
    (:5
      (return "NewEnumerator2")))
  (return "NewEnumerator1"))

(fn RushdownPlayer
  (for _index (range 0 (Variables|RushdownEnemySpawning|GetRushdownEnemiesToSpawn))
    (CallFunction|PlaceEnemyinWorld "/Game/Enemies/Blueprints/BP_RushdownEnemy.BP_RushdownEnemy_C"))
  (Variables|RushdownEnemySpawning|SetRushdownEnemyTimer (Math|Random|RandomFloatinRangefromStream (Variables|Default|GetRandomStream) 25.0 45.0))
  (Math|Integer|IncrementInt (Variables|RushdownEnemySpawning|GetRushdownEnemiesToSpawn)))

(fn PlaceWeaponUpgrade
  (params (Transform :type Transform))
  (bind _returnvalue (Game|SpawnActorfromClass "/Game/Blueprints/BP_WeaponUpgrade.BP_WeaponUpgrade_C" Transform "Undefined" "MultiplyWithRoot" 0 0))
  (return _returnvalue))

(fn SpawnUpgradeEnemy
  (bind _returnvalue (CallFunction|GetSpawnLocation (Variables|Default|GetRandomStream)))
  (bind _returnvalue_2 (Game|SpawnActorfromClass "/Game/Enemies/Blueprints/BP_Miniboss.BP_Miniboss_C" _returnvalue "Undefined" "MultiplyWithRoot" 0 0))
  (Class|KismetMathLibrary|SeedRandomStream (Variables|Default|GetRandomStream))
  (return _returnvalue_2))

(fn SetWeaponUpgrade
  (params (ActorIn :type BP%20Miniboss%20Object%20Reference))
  (Utilities|IsValid ActorIn
    (:Is%20Valid
      (bind _outputfiringmode (CallFunction|GetWeaponUpgradetoSpawn))
      (Variables|/Game/Enemies/Blueprints/BP_Miniboss.BP_Miniboss_C|SetUpgradeToDrop ActorIn _outputfiringmode))
    (:Is%20Not%20Valid
      (Development|PrintString "INVALID"))))

(fn GetWeaponUpgradetoSpawn
  (bind _returnvalue (|GetNumEnumEntries))
  (bind _upgradeincrement (Variables|Default|GetUpgradeIncrement))
  (bind _returnvalue_2 (- _returnvalue 1))
  (return (select (>= _upgradeincrement _returnvalue_2) "NewEnumerator4" (Utilities|Select :Index (Math|Integer|Clamp(Integer) _upgradeincrement 1 _returnvalue_2) :Option%200 "NewEnumerator0" :Option%201 "NewEnumerator1" :Option%202 "NewEnumerator2" :Option%203 "NewEnumerator3"))))